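; Throwaway Blueprint that deliberately wastes frame time, marked by an author comment as not to be used.
; Every Tick runs two identical loops of about a thousand visibility line traces between random unit vectors near the world origin.
; Each trace prints several hit result fields as strings, so the cost grows with both tracing and on-screen logging.
; BeginPlay, overlap and construction script are empty.
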(event `self.ReceiveTick`
  (params (DeltaSeconds :type "Float (single-precision)"))
  ; This blueprint is horseshit, don't use this.
  (for _ (range 1001)
    (bind _outhit (`KismetSystemLibrary.LineTraceSingle` (`KismetMathLibrary.RandomUnitVector`) (`KismetMathLibrary.RandomUnitVector`) "TraceTypeQuery1"))
    (`KismetSystemLibrary.PrintString` (`KismetStringLibrary.Conv_DoubleToString` (`.Time` (`GameplayStatics.BreakHitResult` _outhit))))
    (`KismetSystemLibrary.PrintString` (`KismetStringLibrary.Conv_DoubleToString` (`.Distance` (`GameplayStatics.BreakHitResult` _outhit))))
    (`KismetSystemLibrary.PrintString` (`KismetStringLibrary.Conv_VectorToString` (`.Location` (`GameplayStatics.BreakHitResult` _outhit))))
    (`KismetSystemLibrary.PrintString` (`KismetStringLibrary.Conv_VectorToString` (`.ImpactPoint` (`GameplayStatics.BreakHitResult` _outhit))))
    (`KismetSystemLibrary.PrintString` (`KismetStringLibrary.Conv_VectorToString` (`.Normal` (`GameplayStatics.BreakHitResult` _outhit))))
    (`KismetSystemLibrary.PrintString` (`KismetStringLibrary.Conv_VectorToString` (`.ImpactNormal` (`GameplayStatics.BreakHitResult` _outhit)))))
  (for _ (range 1001)
    (bind _outhit_2 (`KismetSystemLibrary.LineTraceSingle` (`KismetMathLibrary.RandomUnitVector`) (`KismetMathLibrary.RandomUnitVector`) "TraceTypeQuery1"))
    (`KismetSystemLibrary.PrintString` (`KismetStringLibrary.Conv_DoubleToString` (`.Time` (`GameplayStatics.BreakHitResult` _outhit_2))))
    (`KismetSystemLibrary.PrintString` (`KismetStringLibrary.Conv_DoubleToString` (`.Distance` (`GameplayStatics.BreakHitResult` _outhit_2))))
    (`KismetSystemLibrary.PrintString` (`KismetStringLibrary.Conv_VectorToString` (`.Location` (`GameplayStatics.BreakHitResult` _outhit_2))))
    (`KismetSystemLibrary.PrintString` (`KismetStringLibrary.Conv_VectorToString` (`.ImpactPoint` (`GameplayStatics.BreakHitResult` _outhit_2))))
    (`KismetSystemLibrary.PrintString` (`KismetStringLibrary.Conv_VectorToString` (`.Normal` (`GameplayStatics.BreakHitResult` _outhit_2))))
    (`KismetSystemLibrary.PrintString` (`KismetStringLibrary.Conv_VectorToString` (`.ImpactNormal` (`GameplayStatics.BreakHitResult` _outhit_2))))))

(fn `UserConstructionScript`)